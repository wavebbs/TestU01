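; BP_MC01 is a player character Blueprint that exposes attack hitbox control and a bullet-time test.
; AttackColliderON and AttackColliderOff open and close the AttackHitBox attack window, with both sides of the attack-data validity check making the same argument-less begin call.
; The Jump input action calls TestBulletTime on MyTimeScaleTest instead of jumping.
; Tick switches on CurrentState, but no state has logic attached.
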(event `self.ReceiveTick`
  (params (DeltaSeconds :type "Float (single-precision)"))
  (switch `ECharacterAnimState` (`self.CurrentState`)))

(event `EnhancedInput|/Game/Input/Actions/IA_Jump`
  (params (ActionValue :type Boolean) (ElapsedSeconds :type "Float (double-precision)") (TriggeredSeconds :type "Float (double-precision)") (InputAction :type "InputAction Object Reference" :default "/Game/Input/Actions/IA_Jump.IA_Jump"))
  (:`Triggered`
    (`MyTimeScaleTestComponent.TestBulletTime` (`self.MyTimeScaleTest`))))

(fn `AttackColliderOff`
  (`AttackHitBoxComponent.EndAttackWindow` (`self.AttackHitBox`)))

(fn `AttackColliderON`
  (params (`In Attack Data` :type "Object Object Reference"))
  (if (`KismetSystemLibrary.IsValid` `In Attack Data`)
    (`AttackHitBoxComponent.BeginAttackWindow` (`self.AttackHitBox`) null)
    (else
      (`AttackHitBoxComponent.BeginAttackWindow` (`self.AttackHitBox`) null))))

(fn `UserConstructionScript`)